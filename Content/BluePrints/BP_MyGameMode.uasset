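; Game mode that runs the match flow: it shows the player HUD at start and restores game-only input.
; AddScore counts pickups and calls GameResult as a clear at five points.
; GameResult shows the clear or game-over widget and plays a result sound cue switched by a bool parameter.
; Tick counts all BP_Light actors each frame and sets Exploding once PassedLights matches that count.
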(event `self.ReceiveBeginPlay`
  (bind _returnvalue (`GameplayStatics.GetPlayerController` 0))
  ;[1 1 1] ライフゲージを表示
  (bind _returnvalue_2 (`|CreateWidget` "/Game/UMG/PlayerUI.PlayerUI_C")) ; 選択したウィジェットをブループリント中に作成
  (`UserWidget.AddToViewport` _returnvalue_2 0) ; 画面上にウィジェットを表示
  ;;[1 1 1] 入力をゲームに戻す P359
  (`/Engine/EditorBlueprintResources/StandardMacros.IsValid` _returnvalue
    (:`Is Valid`
      (`WidgetBlueprintLibrary.SetInputMode_GameOnly` _returnvalue))))

(event `self.ReceiveTick`
  (params (DeltaSeconds :type "Float (single-precision)"))
  ;[1 1 1] 全てのライトを通過したら爆発フラグをＯｎにする
  (bind _outactors (`GameplayStatics.GetAllActorsOfClass` "/Game/BluePrints/BP_Light.BP_Light_C")) ; レベル内にあるライト（BP_Light）を全て取得し配列にする
  (bind _output_get (set `self.NumbersOfLights` (`KismetArrayLibrary.Array_Length` _outactors))) ; 全てのライトの個数
  (if (== _output_get (`self.PassedLights`))
    (set `self.Exploding` true) ; 変数ExplodingをTrueにする
  ))

(event `GameResult`
  (params (Clear :type Boolean))
  ;[1 1 1] CrearUIまたはGameOverUIを表示 P349
  (bind _returnvalue (`|CreateWidget` (select `bool` Clear :`false` "/Game/UMG/GameOverUI.GameOverUI_C" :`true` "/Game/UMG/ClearUI.ClearUI_C" :!type "UserWidget Class Reference")))
  ;;[1 1 1] サウンドキューを再生する P371
  (set `self.ClearFlag` (select `bool` Clear :`true` true))
  (`UserWidget.AddToViewport` _returnvalue 0)
  (bind _returnvalue_2 (`GameplayStatics.SpawnSoundAtLocation` "/Game/Audio/ResultCue.ResultCue" (0.0 0.0 0.0) (struct) 1.0 1.0 0.0 null null))
  (`AudioComponent.SetBoolParameter` _returnvalue_2 "Result" (`self.ClearFlag`)))

(fn `AddScore`
  ;[1 1 1] スコア加算の関数 P296
  (bind _output_get (set `self.TotalScore` (+ (`self.TotalScore`) 1)))
  ;;[1 1 1] 5つ以上アイテムを取ったらクリアにする P357
  (if (>= _output_get 5)
    (`self.GameResult` true)))

(fn `UserConstructionScript`)