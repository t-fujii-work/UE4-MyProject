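; BP_Light is a point light actor that turns on when a character enters its box and counts toward the number of lights passed.
; The first box overlap, gated by DoOnce with no filter on the overlapping actor, sets the Lighting flag and increments PassedLights on BP_MyGameMode.
; Tick applies Lighting to the PointLight's visibility every frame.
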(event `self.ReceiveTick`
  (params (DeltaSeconds :type "Float (single-precision)"))
  ;[1 1 1] 変数LightingでライトをOn/Off  P177
  (`SceneComponent.SetVisibility` (`self.PointLight`) (`self.Lighting`) false) ; アクタの可視化を行う。\nここではライトを点灯するために使用。\nLightingをTrueにするとライトが点灯する。
)

(event `self.Box.OnComponentBeginOverlap`
  (params (OverlappedComponent :type "PrimitiveComponent Object Reference") (OtherActor :type "Actor Object Reference") (OtherComp :type "PrimitiveComponent Object Reference") (OtherBodyIndex :type Integer) (bFromSweep :type Boolean) (SweepResult :type "HitResult Structure (by ref)"))
  ;[1 1 1] キャラクターが範囲に入ってきたら点灯させる P179
  (`/Engine/EditorBlueprintResources/StandardMacros.DoOnce` false ; 一度だけ実行
    (:`Completed`
      (set `self.Lighting` true)
      ;[1 1 1] ライトを通った時にカウントする
      (bind _asbp_my_game_mode (cast `/Game/BluePrints/BP_MyGameMode` (`GameplayStatics.GetGameMode`))) ; BP_MyGameModeクラスにアクセスするためキャストを行う
      (set `/Game/BluePrints/BP_MyGameMode.PassedLights` (+ (`/Game/BluePrints/BP_MyGameMode.PassedLights` _asbp_my_game_mode) 1) _asbp_my_game_mode))))

(fn `UserConstructionScript`)